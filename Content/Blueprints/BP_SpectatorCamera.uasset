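; BP_SpectatorCamera handles the pause menu toggle for the spectator camera, with no camera logic in its graphs.
; BeginPlay creates and caches a WBP_Pause widget, which the Pause Game input adds or removes while toggling game pause and mouse cursor.
; An invalid widget is only recreated on that press, without pausing.
; Unpausing sets game-only input; the UI-only input node is unconnected, and a debug "Hello" print remains.
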(event `self.ReceiveBeginPlay`
  ;[1 1 1] Pause Game
  (bind _returnvalue (`|CreateWidget` "/Game/Blueprints/Widget/WBP_Pause.WBP_Pause_C" :!label _label))
  (set `self.PauseMenuRef` _returnvalue))

(event `InputAction|Pause Game` :paused true
  (params (Key :type "Key Structure"))
  (bind _returnvalue (`GameplayStatics.GetPlayerController` 0))
  (bind _pausemenuref (`self.PauseMenuRef`))
  ;[1 1 1] Pause Game
  (:`Pressed`
    (`KismetSystemLibrary.PrintString` "Hello")
    (`/Engine/EditorBlueprintResources/StandardMacros.IsValid` (`self.PauseMenuRef`)
      (:`Is Valid`
        (if (`GameplayStatics.IsGamePaused`)
          (`Widget.RemoveFromParent` _pausemenuref)
          (`GameplayStatics.SetGamePaused` false)
          (set `PlayerController.bShowMouseCursor` false _returnvalue)
          (`WidgetBlueprintLibrary.SetInputMode_GameOnly` _returnvalue)
          (else
            (`UserWidget.AddToViewport` _pausemenuref 0)
            (`GameplayStatics.SetGamePaused` true)
            (set `PlayerController.bShowMouseCursor` true _returnvalue))))
      (:`Is Not Valid`
        (goto _label)))))

(fn `UserConstructionScript`)